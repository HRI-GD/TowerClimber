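; BP_Pig is a pig character that turns 180 degrees at cliff edges and on capsule hits; nothing here drives its walking.
; While grounded, Tick line-traces downward from a point offset along world X by the forward vector's X, and flips yaw when no floor is found.
; Capsule hits flip it through a DoOnce that resets after a short delay, debouncing repeated contacts.
; Debug prints and trace drawing remain on.
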(event `self.ReceiveTick`
  (params (DeltaSeconds :type "Float (single-precision)"))
  (if (not (`NavMovementInterface.IsFalling` (`self.CharacterMovement`)))
    (bind _returnvalue (`self.DetectCliff` (`self.K2_GetActorLocation`) (`self.GetActorForwardVector`)))
    (if (not _returnvalue)
      (`self.RotateChar`)
      (`KismetSystemLibrary.PrintString` "Cliff"))))

(event `self.CapsuleComponent.OnComponentHit`
  (params (HitComponent :type "PrimitiveComponent Object Reference") (OtherActor :type "Actor Object Reference") (OtherComp :type "PrimitiveComponent Object Reference") (NormalImpulse :type "Vector Structure") (Hit :type "HitResult Structure (by ref)"))
  (`/Engine/EditorBlueprintResources/StandardMacros.DoOnce` false :!label _label
    (:`Completed`
      (`self.RotateChar`)
      (`KismetSystemLibrary.PrintString` "Wall")
      (`KismetSystemLibrary.Delay` 0.2)
      (goto _label :!via `Reset`))))

(fn `DetectCliff`
  (params (Location :type "Vector Structure") (`Forward Vector` :type "Vector Structure"))
  (returns (ReturnValue :type Boolean))
  (bind (_outhit _returnvalue) (`KismetSystemLibrary.LineTraceSingle` :`Start` (+ Location (* `Forward Vector` (30.0 0.0 0.0))) :`End` (- (+ Location (* `Forward Vector` (30.0 0.0 0.0))) (0.0 0.0 100.0)) :`TraceChannel` "TraceTypeQuery1" :`DrawDebugType` "ForDuration" :`DrawTime` 0.01))
  (return _returnvalue))

(fn `RotateChar`
  (bind (_returnvalue_roll _returnvalue_pitch _returnvalue_yaw) (`KismetMathLibrary.BreakRotator` (`self.K2_GetActorRotation`)))
  (`self.K2_SetActorRotation` (`KismetMathLibrary.MakeRotator` 0.0 0.0 (- _returnvalue_yaw 180.0))))

(fn `UserConstructionScript`
  (`parent.UserConstructionScript`))